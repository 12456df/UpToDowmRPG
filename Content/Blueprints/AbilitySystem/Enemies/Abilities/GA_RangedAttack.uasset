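; Enemy gameplay ability that performs a ranged attack by firing a projectile at the avatar's combat target.
; On activation it turns the avatar toward the target through interface messages and plays a random attack montage.
; A gameplay event matching a montage tag triggers a combat socket lookup, projectile spawn and debug sphere.
; The ability ends after spawning without stopping the montage, or when the montage completes, is interrupted or cancelled.
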(event `self.K2_ActivateAbility`
  (bind _returnvalue (`self.GetAvatarActorFromActorInfo`))
  (bind _returnvalue_2 (message `CombatInterface.GetCombatTarget` _returnvalue))
  (bind _returnvalue_3 (message `CombatInterface.GetAttackMontages` _returnvalue))
  (message `CombatInterface.UpdateFacingRotation` _returnvalue (`Actor.K2_GetActorLocation` _returnvalue_2))
  (bind _outitem (`KismetArrayLibrary.Array_Random` _returnvalue_3))
  (`AbilityTask_PlayMontageAndWait.CreatePlayMontageAndWaitProxy` "None" (break `TaggedMontage` _outitem) 1.0 "None" false
    (:`then`
      (`AbilityTask_WaitGameplayEvent.WaitGameplayEvent` (`.MontageTag` (break `TaggedMontage` _outitem)) null
        (:`then`
          (message `CombatInterface.GetCombatSocketLocation` (`self.GetAvatarActorFromActorInfo`) (`.MontageTag` (break `TaggedMontage` _outitem)))
          (bind _returnvalue_4 (message `CombatInterface.GetCombatTarget` (`self.GetAvatarActorFromActorInfo`)))
          (`self.SpawnProjectile` (`Actor.K2_GetActorLocation` _returnvalue_4))
          (`KismetSystemLibrary.DrawDebugSphere` (0.0 0.0 0.0) 10.0 12 (struct :`R` 1.0 :`G` 1.0 :`B` 1.0 :`A` 1.0) 0.5)
          (`self.K2_EndAbility`))))
    (:`OnCompleted`
      (`self.K2_EndAbility` :!label _label))
    (:`OnInterrupted`
      (goto _label))
    (:`OnCancelled`
      (goto _label))))