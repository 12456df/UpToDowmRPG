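; BP_FireBall is the Fire Blast ability's projectile, which flies out and returns like a boomerang before exploding.
; StartOutgoingTimeline chains two timelines, lerping forward to an apex, then back toward ReturnToActor's live location.
; Within DistanceToExplore of that actor, it calls OnHit, sets radial damage, knockback and death impulse params for nearby live players except its owner, then destroys itself.
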(event `self.ReceiveBeginPlay`)

(event `self.StartOutgoingTimeline`
  (bind _explosiondamageparams (`self.ExplosionDamageParams`))
  (bind _array (`|MakeArray` (`self.GetOwner`)))
  (bind _output_get (set `self.StartLocation` (`self.K2_GetActorLocation`)))
  (set `self.ApexLocation` (+ _output_get (* (`self.GetActorForwardVector`) (`self.Speed`))))
  (bind (_direction `_新建轨道_0`) (`Timeline|时间轴`)
    (:`Update`
      (`self.K2_SetActorLocation` (`KismetMathLibrary.VLerp` (`self.StartLocation`) (`self.ApexLocation`) `_新建轨道_0`)))
    (:`Finished`
      (bind (_direction_2 `_新建轨道_0_2`) (`Timeline|时间轴_0`)
        (:`Update`
          (`self.K2_SetActorLocation` (`KismetMathLibrary.VLerp` (`self.ApexLocation`) (`self.K2_GetActorLocation` (`self.ReturnToActor`)) `_新建轨道_0_2`))
          (if (< (`KismetMathLibrary.VSize` (- (`self.K2_GetActorLocation` (`self.ReturnToActor`)) (`self.K2_GetActorLocation`))) (`self.DistanceToExplore`))
            (`self.OnHit`)
            (`KismetArrayLibrary.Array_Add` _array self)
            (bind _outoverlappingactors (`AuraAbilitySystemLibrary.GetLivePlayersWithinRadius` self _array 300.0 (`self.K2_GetActorLocation`)))
            (set `self.Out Overlapping Actors` _outoverlappingactors)
            (`AuraAbilitySystemLibrary.SetIsRadialDamageEffectParam` (`self.ExplosionDamageParams`) true 100.0 350.0 (`self.K2_GetActorLocation`))
            (for _array_element (`self.Out Overlapping Actors`)
              (`AuraAbilitySystemLibrary.SetTargetEffectParamsASC` (`self.ExplosionDamageParams`) (`AbilitySystemBlueprintLibrary.GetAbilitySystemComponent` _array_element))
              (bind _returnvalue (- (`self.K2_GetActorLocation` _array_element) (`self.K2_GetActorLocation`)))
              (`AuraAbilitySystemLibrary.SetKnockbackDirection` _explosiondamageparams _returnvalue 500.0)
              (`AuraAbilitySystemLibrary.SetDeathImpulseDirection` _explosiondamageparams _returnvalue 400.0))
            (`self.K2_DestroyActor`)))))))

(fn `UserConstructionScript`)