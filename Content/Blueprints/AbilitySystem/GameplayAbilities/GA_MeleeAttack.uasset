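; Melee attack gameplay ability that turns the avatar toward its combat target and plays a randomly picked attack montage.
; It waits for the montage's gameplay event tag, then gathers live players in a small sphere at the matching combat socket.
; Non-friendly hits take damage through CauseDamage.
; The ability ends after that hit check or when the montage completes, is interrupted or is cancelled.
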(event `self.K2_ActivateAbility`
  (bind _returnvalue (`self.GetAvatarActorFromActorInfo`))
  (bind _returnvalue_2 (`self.GetAvatarActorFromActorInfo`))
  ;[1 1 1] Get CombatTarget And Play Attack Montage to Target
  (bind _returnvalue_3 (message `CombatInterface.GetCombatTarget` _returnvalue))
  (bind _returnvalue_4 (message `CombatInterface.GetAttackMontages` _returnvalue))
  (message `CombatInterface.UpdateFacingRotation` _returnvalue_3 (`Actor.K2_GetActorLocation` _returnvalue_3))
  (bind _outitem (`KismetArrayLibrary.Array_Random` _returnvalue_4))
  (`AbilityTask_PlayMontageAndWait.CreatePlayMontageAndWaitProxy` "None" (break `TaggedMontage` _outitem)
    (:`then`
      (`AbilityTask_WaitGameplayEvent.WaitGameplayEvent` (`.MontageTag` (break `TaggedMontage` _outitem)) null
        (:`EventReceived`
          ;[1 1 1] After Receive GameplayEvent,Use Weapon SocketLocation to Creat a Sphere to Detective Who is be Hit
          (bind _returnvalue_5 (message `CombatInterface.GetCombatSocketLocation` _returnvalue_2 (`.MontageTag` (break `TaggedMontage` _outitem))))
          (bind _outoverlappingactors (`AuraAbilitySystemLibrary.GetLivePlayersWithinRadius` _returnvalue_2 (`|MakeArray` _returnvalue_2) 45.0 _returnvalue_5))
          ;;[1 1 1] Cause Damage
          (for _array_element _outoverlappingactors
            (if (`AuraAbilitySystemLibrary.IsNotFriend` _array_element (`self.GetAvatarActorFromActorInfo`))
              (`self.CauseDamage` _array_element)))
          (`self.K2_EndAbility`))))
    (:`OnCompleted`
      (`self.K2_EndAbility` :!label _label))
    (:`OnInterrupted`
      (goto _label))
    (:`OnCancelled`
      (goto _label))))